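; Side-scrolling Paper2D player character with walking, jumping, crouching and wall jumping, using a replicated sprite.
; Move input drives movement along world X, turns the controller left or right and refreshes the flipbook through a state-selection function using falling, moving and crouching flags.
; Jumping while airborne traces through the capsule along its forward axis and launches away from any wall hit.
; Launching arms a short delay in airborne movement handling.
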(event `InputAction|Jump`
  (params (Key :type "Key Structure"))
  ;[1 1 1] Jumping
  (:`Pressed`
    (`self.Jump`)
    (if (`NavMovementComponent.IsFalling` (`self.CharacterMovement`))
      (`self.WallJump`))))

(event `self.ReceiveBeginPlay`
  ;[1 1 1] Replication
  (`ActorComponent.SetIsReplicated` (`self.Sprite`) true))

(event `InputAxis|MoveRight`
  (params (AxisValue :type "Float (single-precision)"))
  ;[1 1 1] Movement
  (`self.AddMovementInput` (1.0 0.0 0.0) AxisValue)
  (`self.UpdateAnimation`)
  (if (`NavMovementComponent.IsFalling` (`self.CharacterMovement`))
    (`KismetSystemLibrary.Delay` (stale `self.OnLaunched` _output_get))
    (set `self.Delay` 0.0))
  (`/Engine/EditorBlueprintResources/StandardMacros.CompareFloat` AxisValue
    (:`>`
      (`Controller.SetControlRotation` (`self.GetController`) (`KismetMathLibrary.MakeRotator` 0.0))
      (set `self.Orientation` 0))
    (:`<`
      (`Controller.SetControlRotation` (`self.GetController`) (`KismetMathLibrary.MakeRotator` 0.0 0.0 180.0))
      (set `self.Orientation` 0))))

(event `UpdateAnimation`
  ;[1 1 1] Flipbook Change
  (set `self.Is Moving` (> (`KismetMathLibrary.VSize` (`self.GetVelocity`)) 0.0))
  (set `self.IsFalling` (`NavMovementComponent.IsFalling` (`self.CharacterMovement`)))
  (set `self.IsChrouching` (`NavMovementComponent.IsCrouching` (`self.CharacterMovement`)))
  (bind _outputflibook (`self.Animation State Machine` (`self.IsFalling`) (`self.Is Moving`) (`self.IsChrouching`)))
  (`PaperFlipbookComponent.SetFlipbook` (`self.Sprite`) _outputflibook))

(event `self.OnLaunched`
  (params (LaunchVelocity :type "Vector Structure") (bXYOverride :type Boolean) (bZOverride :type Boolean))
  ;[1 1 1] Movement
  (bind _output_get (set `self.Delay` 0.8)))

(event `WallJump`
  (bind _returnvalue (`self.GetActorForwardVector`))
  (bind _returnvalue_x (`KismetMathLibrary.BreakVector` (`self.K2_GetActorLocation`)))
  ;[1 1 1] Wall Jumping
  (bind (_outhit _returnvalue_2) (`KismetSystemLibrary.LineTraceSingle` (- (`self.K2_GetActorLocation`) (* _returnvalue (+ (`CapsuleComponent.GetScaledCapsuleRadius` (`self.CapsuleComponent`)) 15.0))) (+ (`self.K2_GetActorLocation`) (* _returnvalue (+ (`CapsuleComponent.GetScaledCapsuleRadius` (`self.CapsuleComponent`)) 15.0))) "TraceTypeQuery1" true))
  (if _returnvalue_2
    (`self.LaunchCharacter` (`KismetMathLibrary.MakeVector` (* (`KismetMathLibrary.SignOfFloat` (- _returnvalue_x (.x (`.Location` (`GameplayStatics.BreakHitResult` _outhit))))) 600.0) 0.0 (`CharacterMovementComponent.JumpZVelocity` (`self.CharacterMovement`))) true true)
    (`/Engine/EditorBlueprintResources/StandardMacros.CompareFloat` (select `byte` (`self.Orientation`) :`0` 0.0 :`1` 0.0 :!type "Float (single-precision)")
      (:`>`
        (`Controller.SetControlRotation` (`self.GetController`) (`KismetMathLibrary.MakeRotator` 0.0 0.0 180.0)))
      (:`<`
        (`Controller.SetControlRotation` (`self.GetController`) (`KismetMathLibrary.MakeRotator` 0.0))))))

(event `InputAction|Crouch`
  (params (Key :type "Key Structure"))
  ;[1 1 1] Crouch?
  (:`Pressed`
    (`self.Crouch`))
  (:`Released`
    (`self.UnCrouch`)))

(fn `Animation State Machine`
  (params (IsFalling :type Boolean) (IsMoving :type Boolean) (IsCrouching :type Boolean))
  (returns (OutputFlibook :type "PaperFlipbook Object Reference"))
  (locals (AnimationState :type Byte) (IsFalLoc :type Boolean) (IsMovLocal :type Boolean) (IsCrouchLocal :type Boolean))
  (set `local.IsFalLoc` IsFalling)
  (set `local.IsMovLocal` IsMoving)
  (set `local.IsCrouchLocal` IsCrouching)
  (if (`local.IsCrouchLocal`)
    (set `local.AnimationState` 0)
    (elif (`local.IsFalLoc`)
      (set `local.AnimationState` 0)
      (elif (`local.IsMovLocal`)
        (set `local.AnimationState` 0)
        (else
          (set `local.AnimationState` 0)))))
  (return (select `byte` (`local.AnimationState`) :`0` null :`1` null :`2` null :`3` null :!type "PaperFlipbook Object Reference")))

(fn `UserConstructionScript`)