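; PlayerRed is a side-scrolling 2D player character with horizontal movement, facing flips, jump and dash, using a replicated flipbook sprite.
; Axis input and dash events refresh animation through a macro-built state machine that prioritises Dashing, Jumping, Running, then Idle.
; Dash plays a timeline that sweeps the capsule along its forward vector, switching the movement plane constraint from Y to Z until it finishes.
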(event `self.ReceiveBeginPlay`
  ;[1 1 1] Replication
  (`ActorComponent.SetIsReplicated` (`self.Sprite`) true))

(event `UpdateAnimation`
  ;[1 1 1] AnimationHandling
  (bind _output_get (set `self.IsMoving` (> (`KismetMathLibrary.VSize` (`self.GetVelocity`)) 0.0)))
  (bind _output_get_2 (set `self.IsFalling` (`NavMovementComponent.IsFalling` (`self.CharacterMovement`))))
  (bind _outputflipbook (`self.AnimationStateMachine` _output_get_2 _output_get (`self.IsDashing`)))
  (`PaperFlipbookComponent.SetFlipbook` (`self.Sprite`) _outputflipbook))

(event `InputAxis|Horizontal`
  (params (AxisValue :type "Float (single-precision)"))
  (`self.AddMovementInput` (1.0 0.0 0.0) AxisValue)
  (`self.UpdateAnimation`)
  (`/Engine/EditorBlueprintResources/StandardMacros.CompareFloat` AxisValue
    (:`>`
      (`self.K2_SetActorRotation` (struct)))
    (:`<`
      (`self.K2_SetActorRotation` (struct :`Yaw` 180.0)))))

(event `InputAction|Jump`
  (params (Key :type "Key Structure"))
  (:`Pressed`
    (`self.Jump`)))

(event `InputAction|Dash`
  (params (Key :type "Key Structure"))
  (:`Pressed`
    (set `self.IsDashing` true)
    (`self.UpdateAnimation`)
    (`MovementComponent.SetPlaneConstraintAxisSetting` (`self.CharacterMovement`) "Z")
    (bind (_direction _dashduration) (`Timeline|DashTime` :!via `PlayFromStart`)
      (:`Update`
        (`SceneComponent.K2_AddWorldOffset` (`self.CapsuleComponent`) (`KismetMathLibrary.MakeVector` (.x (* (`SceneComponent.GetForwardVector` (`self.CapsuleComponent`)) _dashduration)) 0.0 (.z (* (`SceneComponent.GetForwardVector` (`self.CapsuleComponent`)) _dashduration))) true false))
      (:`Finished`
        (set `self.IsDashing` false)
        (`self.UpdateAnimation`)
        (`MovementComponent.SetPlaneConstraintAxisSetting` (`self.CharacterMovement`) "Y")))))

(fn `AnimationStateMachine`
  (params (IsFalling :type Boolean) (IsMoving :type Boolean) (IsDashing :type Boolean))
  (returns (OutputFlipBook :type "PaperFlipbook Object Reference"))
  (locals (AnimationState :type "/Game/Data/AnimationState Enum") (IsFallingL :type Boolean) (IsMovingL :type Boolean) (IsDashingL :type Boolean))
  ;[1 1 1] Collect Data
  (set `local.IsFallingL` IsFalling)
  (set `local.IsMovingL` IsMoving)
  (set `local.IsDashingL` IsDashing)
  ;[1 1 1] TestData
  (if (`local.IsDashingL`)
    ;[1 1 1] SetAnimationState
    (set `local.AnimationState` "NewEnumerator3")
    (elif (`local.IsFallingL`)
      (set `local.AnimationState` "NewEnumerator2")
      (elif (`local.IsMovingL`)
        (set `local.AnimationState` "NewEnumerator1")
        (else
          (set `local.AnimationState` "NewEnumerator0")))))
  (return (select `/Game/Data/AnimationState` (`local.AnimationState`) :`NewEnumerator0` (`self.IdleFlipBook`) :`NewEnumerator1` (`self.RunFlipBook`) :`NewEnumerator2` (`self.JumpFlipBook`) :`NewEnumerator3` (`self.DashFlipBook`))))

(fn `UserConstructionScript`)