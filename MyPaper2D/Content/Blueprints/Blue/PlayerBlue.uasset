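; Paper2D side-scrolling player character with running, jumping, wall jumps, dashing and an aimable cannon that fires BlueProjectile.
; BeginPlay creates a local player and picks colored flipbooks from its controller ID.
; A priority state machine (dash, jump, run, idle) selects the sprite flipbook on move and dash updates.
; Dash sweeps the capsule through a timeline while constrained on Z, and wall jumps use a line trace to launch away from walls.
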(event `self.ReceiveBeginPlay`
  ;[1 1 1] Replication
  (bind _returnvalue (`GameplayStatics.CreatePlayer` -1))
  (`ActorComponent.SetIsReplicated` (`self.Sprite`) true)
  (bind _returnvalue_2 (`GameplayStatics.GetPlayerControllerID` _returnvalue))
  (bind _output_get (set `self.PlayerId` _returnvalue_2))
  (`self.SelectPlayerColor` _output_get)
  (`PaperFlipbookComponent.SetFlipbook` (`self.Canon`) (`self.CanonFlipbook`)))

(event `UpdateAnimation`
  ;[1 1 1] AnimationHandling
  (bind _output_get (set `self.IsMoving` (> (`KismetMathLibrary.VSize` (`self.GetVelocity`)) 0.0)))
  (bind _output_get_2 (set `self.IsFalling` (`NavMovementComponent.IsFalling` (`self.CharacterMovement`))))
  (bind _outputflipbook (`self.AnimationStateMachine` _output_get_2 _output_get (`self.IsDashing`)))
  (`PaperFlipbookComponent.SetFlipbook` (`self.Sprite`) _outputflipbook))

(event `InputAxis|Horizontal`
  (params (AxisValue :type "Float (single-precision)"))
  ;[1 1 1] Running
  (`self.Move` AxisValue))

(event `InputAction|Jump`
  (params (Key :type "Key Structure"))
  ;[1 1 1] Jump/Wall Jump Check
  (:`Pressed`
    (`self.JumpEvent`)))

(event `JumpEvent`
  ;[1 1 1] Jump/Wall Jump Check
  (`self.Jump`)
  (if (`NavMovementComponent.IsFalling` (`self.CharacterMovement`))
    (`self.WallJumping`)))

(event `self.OnLaunched`
  (params (LaunchVelocity :type "Vector Structure") (bXYOverride :type Boolean) (bZOverride :type Boolean))
  ;[1 1 1] Running
  (bind _output_get (set `self.Delay` 0.4)))

(event `Move`
  (params (Axis :type "Float (double-precision)"))
  ;[1 1 1] Running
  (`self.AddMovementInput` (1.0 0.0 0.0) Axis)
  (`self.UpdateAnimation`)
  (if true
    (`KismetSystemLibrary.Delay` (stale `self.OnLaunched` _output_get))
    (set `self.Delay` 0.0))
  (`/Engine/EditorBlueprintResources/StandardMacros.CompareFloat` Axis
    (:`>`
      (`self.K2_SetActorRotation` (struct))
      (set `self.Orientation` "NewEnumerator0"))
    (:`<`
      (`self.K2_SetActorRotation` (struct :`Yaw` 180.0))
      (set `self.Orientation` "NewEnumerator1"))))

(event `Fire`
  (bind _returnvalue (`SceneComponent.GetForwardVector` (`self.Canon`)))
  ;[1 1 1] Fire
  (bind _returnvalue_2 (`|SpawnActorFromClass` "/Game/Blueprints/Blue/BlueProjectile.BlueProjectile_C" (`KismetMathLibrary.Conv_VectorToTransform` (`SceneComponent.GetSocketLocation` (`self.Canon`) "BulletSpawn")) "AdjustIfPossibleButAlwaysSpawn" "OverrideRootScale" null null))
  (bind _projectilemovement (`/Game/Blueprints/Blue/BlueProjectile.ProjectileMovement` _returnvalue_2))
  (`ActorComponent.Activate` _projectilemovement false)
  (`ProjectileMovementComponent.SetVelocityInLocalSpace` _projectilemovement (* _returnvalue 1000.0))
  (`self.K2_SetActorRotation` _returnvalue_2 (`KismetMathLibrary.Conv_VectorToRotator` _returnvalue) false))

(event `InputAction|Dash`
  (params (Key :type "Key Structure"))
  ;[1 1 1] Dash
  (:`Pressed`
    (`self.Dash`)))

(event `InputAction|Fire`
  (params (Key :type "Key Structure"))
  ;[1 1 1] Fire
  (:`Pressed`
    (`self.Fire`)))

(event `Dash`
  ;[1 1 1] Dash
  (set `self.IsDashing` true)
  (`self.UpdateAnimation`)
  (`MovementComponent.SetPlaneConstraintAxisSetting` (`self.CharacterMovement`) "Z")
  (bind (_direction _dashduration) (`Timeline|DashTime` :!via `PlayFromStart`)
    (:`Update`
      (`SceneComponent.K2_AddWorldOffset` (`self.CapsuleComponent`) (`KismetMathLibrary.MakeVector` (.x (* (`SceneComponent.GetForwardVector` (`self.CapsuleComponent`)) _dashduration)) 0.0 (.z (* (`SceneComponent.GetForwardVector` (`self.CapsuleComponent`)) _dashduration))) true false))
    (:`Finished`
      (set `self.IsDashing` false)
      (`self.UpdateAnimation`)
      (`MovementComponent.SetPlaneConstraintAxisSetting` (`self.CharacterMovement`) "Y"))))

(event `WallJumping`
  (bind _returnvalue (`self.GetActorForwardVector`))
  (bind _returnvalue_x (`KismetMathLibrary.BreakVector` (`self.K2_GetActorLocation`)))
  ;[1 1 1] Wall Jumping
  (bind (_outhit _returnvalue_2) (`KismetSystemLibrary.LineTraceSingle` (- (`self.K2_GetActorLocation`) (* _returnvalue (+ (`CapsuleComponent.GetScaledCapsuleRadius` (`self.CapsuleComponent`)) 15.0))) (+ (`self.K2_GetActorLocation`) (* _returnvalue (+ (`CapsuleComponent.GetScaledCapsuleRadius` (`self.CapsuleComponent`)) 15.0))) "TraceTypeQuery1"))
  (if _returnvalue_2
    (`self.LaunchCharacter` (`KismetMathLibrary.MakeVector` (* (`KismetMathLibrary.SignOfFloat` (- _returnvalue_x (.x (`.Location` (`GameplayStatics.BreakHitResult` _outhit))))) 600.0) 0.0 (`CharacterMovementComponent.JumpZVelocity` (`self.CharacterMovement`))) true true)
    (`/Engine/EditorBlueprintResources/StandardMacros.CompareFloat` (select `/Game/Imports/Imports/Data/RightLeft` (`self.Orientation`) :`NewEnumerator0` 1.0 :`NewEnumerator1` -1.0 :!type "Float (single-precision)")
      (:`>`
        (`self.K2_SetActorRotation` (struct :`Yaw` 180.0)))
      (:`<`
        (`self.K2_SetActorRotation` (struct))))))

(event `InputAxis|GunHorizontal`
  (params (AxisValue :type "Float (single-precision)"))
  (bind _returnvalue (`self.K2_GetActorLocation` (`GameplayStatics.GetPlayerCharacter` 0)))
  (`SceneComponent.K2_SetWorldRotation` (`self.Canon`) (`KismetMathLibrary.FindLookAtRotation` _returnvalue (+ (`KismetMathLibrary.MakeVector` AxisValue 0.0 (stale `InputAxis|GunVertical` AxisValue)) _returnvalue)) false false :!label _label))

(event `InputAxis|GunVertical`
  (params (AxisValue :type "Float (single-precision)"))
  (goto _label))

(fn `AnimationStateMachine`
  (params (IsFalling :type Boolean) (IsMoving :type Boolean) (IsDashing :type Boolean))
  (returns (OutputFlipBook :type "PaperFlipbook Object Reference"))
  (locals (AnimationState :type "/Game/Data/AnimationState Enum") (IsFallingL :type Boolean) (IsMovingL :type Boolean) (IsDashingL :type Boolean))
  ;[1 1 1] Collect Data
  (set `local.IsFallingL` IsFalling)
  (set `local.IsMovingL` IsMoving)
  (set `local.IsDashingL` IsDashing)
  ;[1 1 1] TestData
  (if (`local.IsDashingL`)
    ;[1 1 1] SetAnimationState
    (set `local.AnimationState` "NewEnumerator3")
    (elif (`local.IsFallingL`)
      (set `local.AnimationState` "NewEnumerator2")
      (elif (`local.IsMovingL`)
        (set `local.AnimationState` "NewEnumerator1")
        (else
          (set `local.AnimationState` "NewEnumerator0")))))
  (return (select `/Game/Data/AnimationState` (`local.AnimationState`) :`NewEnumerator0` (`self.IdleFlipBook`) :`NewEnumerator1` (`self.RunFlipBook`) :`NewEnumerator2` (`self.JumpFlipBook`) :`NewEnumerator3` (`self.DashFlipBook`))))

(fn `SelectPlayerColor`
  (params (`Player Id` :type Integer))
  (locals (NewLocalVar_0 :type "PaperFlipbookComponent Object Reference" :default null))
  (switch `int` `Player Id`
    (:`Default`
      (set `self.IdleFlipBook` "/Game/FlipBooks/Blue/Idle.Idle" :!label _label)
      (set `self.RunFlipBook` "/Game/FlipBooks/Blue/Run.Run")
      (set `self.JumpFlipBook` "/Game/FlipBooks/Blue/Jump.Jump")
      (set `self.DashFlipBook` "/Game/FlipBooks/Blue/Dash.Dash")
      (set `self.CanonFlipbook` "/Game/FlipBooks/Blue/CannonBlue.CannonBlue")
      (set `self.ProjectileFlipbook` "/Game/FlipBooks/Blue/Projectile.Projectile"))
    (:`0`
      (goto _label))
    (:`1`
      (set `self.IdleFlipBook` "/Game/FlipBooks/Green/Idle.Idle")
      (set `self.RunFlipBook` "/Game/FlipBooks/Green/Run.Run")
      (set `self.JumpFlipBook` "/Game/FlipBooks/Green/Jump.Jump")
      (set `self.DashFlipBook` "/Game/FlipBooks/Green/DashFlipbookGreen.DashFlipbookGreen")
      (set `self.CanonFlipbook` "/Game/FlipBooks/Green/CannonGreen.CannonGreen")
      (set `self.ProjectileFlipbook` "/Game/FlipBooks/Green/Projectile.Projectile"))
    (:`2`
      (set `self.IdleFlipBook` "/Game/FlipBooks/Purple/Idle.Idle")
      (set `self.RunFlipBook` "/Game/FlipBooks/Purple/Run.Run")
      (set `self.JumpFlipBook` "/Game/FlipBooks/Purple/Jump.Jump")
      (set `self.DashFlipBook` "/Game/FlipBooks/Purple/DashFlipbookPurple.DashFlipbookPurple")
      (set `self.CanonFlipbook` "/Game/FlipBooks/Purple/CannonPurple.CannonPurple")
      (set `self.ProjectileFlipbook` "/Game/FlipBooks/Purple/Projectile.Projectile"))
    (:`3`
      (set `self.IdleFlipBook` "/Game/FlipBooks/Red/Idle.Idle")
      (set `self.RunFlipBook` "/Game/FlipBooks/Red/Run.Run")
      (set `self.JumpFlipBook` "/Game/FlipBooks/Red/jump.jump")
      (set `self.DashFlipBook` "/Game/FlipBooks/Red/DashFlipbookRed.DashFlipbookRed")
      (set `self.CanonFlipbook` "/Game/FlipBooks/Red/CannonRed.CannonRed")
      (set `self.ProjectileFlipbook` "/Game/FlipBooks/Red/Projectile.Projectile"))))

(fn `UserConstructionScript`)